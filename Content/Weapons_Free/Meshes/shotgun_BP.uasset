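; Shotgun weapon Blueprint that fires a projectile when shot from the hand holding it.
; Separate left and right shoot input actions each check the GrabComponent's holding hand, so only the matching hand's input fires.
; Both paths share one spawn call that creates a single Projectile at the ShootLocation component's world position and rotation, regardless of collisions.
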(event Input|EnhancedActionEvents|EnhancedInputActionIA_Shoot_Left
  (params (ActionValue :type Boolean) (ElapsedSeconds :type Float%20%28double-precision%29) (TriggeredSeconds :type Float%20%28double-precision%29) (InputAction :type Input%20Action%20Object%20Reference :default "/Game/VRTemplate/Input/Actions/IA_Shoot_Left.IA_Shoot_Left"))
  (bind _shootlocation (Variables|Default|GetShootLocation))
  (if (Utilities|Enum|Equal(Enum) (Default|GetHeldbyHand (Variables|Default|GetGrabComponent)) "Left")
    (Game|SpawnActorfromClass "/Game/VRTemplate/Blueprints/Projectile.Projectile_C" (Math|Transform|MakeTransform (Transformation|GetWorldLocation _shootlocation) (Transformation|GetWorldRotation _shootlocation)) "AlwaysSpawn" "MultiplyWithRoot" 0 0)))

(event Input|EnhancedActionEvents|EnhancedInputActionIA_Shoot_Right
  (params (ActionValue :type Boolean) (ElapsedSeconds :type Float%20%28double-precision%29) (TriggeredSeconds :type Float%20%28double-precision%29) (InputAction :type Input%20Action%20Object%20Reference :default "/Game/VRTemplate/Input/Actions/IA_Shoot_Right.IA_Shoot_Right"))
  (bind _shootlocation (Variables|Default|GetShootLocation))
  (if (Utilities|Enum|Equal(Enum) (Default|GetHeldbyHand (Variables|Default|GetGrabComponent)) "Right")
    (Game|SpawnActorfromClass "/Game/VRTemplate/Blueprints/Projectile.Projectile_C" (Math|Transform|MakeTransform (Transformation|GetWorldLocation _shootlocation) (Transformation|GetWorldRotation _shootlocation)) "AlwaysSpawn" "MultiplyWithRoot" 0 0)))

(fn ConstructionScript)